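; BP_P38_Pawn is a pawn for a P-38 twin-propeller plane that animates its propellers and pushes itself forward automatically.
; Each Tick rolls the left and right propeller components locally by RotateSpeed scaled by world delta seconds, keeping the spin frame-rate independent.
; The same Tick feeds constant movement input along the actor's forward vector, with no player input involved in this graph.
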(event EventBeginPlay)

(event Collision|EventActorBeginOverlap
  (params (OtherActor :type Actor%20Object%20Reference)))

(event EventTick
  (params (DeltaSeconds :type Float%20%28single-precision%29))
  ;[1 1 1] Rotate Left Propeller
  (Transformation|AddLocalRotation (Variables|Default|GetLeft) (Math|Rotator|MakeRotator (* (Utilities|Time|GetWorldDeltaSeconds) (Variables|Speed|GetRotateSpeed)) 0.0 0.0) false false)
  ;[1 1 1] Rotate Right Propeller
  (Transformation|AddLocalRotation (Variables|Default|GetRignt) (Math|Rotator|MakeRotator (* (Utilities|Time|GetWorldDeltaSeconds) (Variables|Speed|GetRotateSpeed)) 0.0 0.0) false false)
  ;[1 1 1] Move P38
  (Pawn|Input|AddMovementInput (Transformation|GetActorForwardVector) 1.0 false))

(fn ConstructionScript)
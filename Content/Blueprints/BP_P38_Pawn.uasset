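; BP_P38_Pawn is a player-flyable P-38 plane pawn that constantly moves forward along its nose.
; Pitch and Roll axes rotate the actor locally at a frame-rate-scaled rate, and Tick feeds forward movement input while spinning both propeller components.
; Boost swaps the FloatingPawnMovement max speed while held, and Fire spawns a BP_Rocket at the Arrow component's transform.
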(event EventTick
  (params (DeltaSeconds :type Float%20%28single-precision%29))
  ;[1 1 1] Rotate Left Propeller
  (Transformation|AddLocalRotation (Variables|Default|GetLeft) (Math|Rotator|MakeRotator (* (Utilities|Time|GetWorldDeltaSeconds) (Variables|Speed|GetRotateSpeed)) 0.0 0.0) false false)
  ;[1 1 1] Rotate Right Propeller
  (Transformation|AddLocalRotation (Variables|Default|GetRignt) (Math|Rotator|MakeRotator (* (Utilities|Time|GetWorldDeltaSeconds) (Variables|Speed|GetRotateSpeed)) 0.0 0.0) false false)
  ;[1 1 1] Move P38
  (Pawn|Input|AddMovementInput (Transformation|GetActorForwardVector) 1.0 false))

(event Input|ActionEvents|InputActionBoost
  (params (Key :type Key%20Structure :default "None"))
  (bind _floatingpawnmovement (Variables|Default|GetFloatingPawnMovement))
  ;[1 1 1] Boost
  (:Pressed
    (Variables|/Script/Engine.FloatingPawnMovement|SetMaxSpeed _floatingpawnmovement (Variables|Speed|GetBoostSpeed)))
  (:Released
    (Variables|/Script/Engine.FloatingPawnMovement|SetMaxSpeed _floatingpawnmovement (Variables|Speed|GetMoveSpeed))))

(event Input|ActionEvents|InputActionFire
  (params (Key :type Key%20Structure :default "None"))
  (:Pressed
    (Game|SpawnActorfromClass "/Game/Blueprints/BP_Rocket.BP_Rocket_C" (Transformation|GetWorldTransform (Variables|Default|GetArrow)) "Undefined" 0 0)))

(event Input|AxisEvents|InputAxisPitch
  (params (AxisValue :type Float%20%28single-precision%29))
  ;[1 1 1] P38 Rotation
  (Transformation|AddActorLocalRotation (Math|Rotator|MakeRotator 0.0 (* (Math|Float|Clamp(Float) AxisValue -1.0 1.0) (Utilities|Time|GetWorldDeltaSeconds) (Variables|Speed|GetDirSpeed)) 0.0) false false))

(event Input|AxisEvents|InputAxisRoll
  (params (AxisValue :type Float%20%28single-precision%29))
  ;[1 1 1] P38 Rotation
  (Transformation|AddActorLocalRotation (Math|Rotator|MakeRotator (* (Math|Float|Clamp(Float) AxisValue -1.0) (Utilities|Time|GetWorldDeltaSeconds) (Variables|Speed|GetDirSpeed)) 0.0 0.0) false false))

(fn ConstructionScript)